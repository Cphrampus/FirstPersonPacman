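; Openable box in the 2.5D lesson that opens when BP_25DPlayer overlaps it and reveals a Note.
; The overlap sets an Open flag, and Tick then loops the Open_Box helper to rotate its Target in small delayed steps until roll reaches -90.
; A DoOnce then raises the Note and briefly unhides the BP_LeftShiftText hint actors.
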(event `self.ReceiveBeginPlay`)

(event `self.ReceiveActorBeginOverlap`
  (params (OtherActor :type "Actor Object Reference"))
  (cast `/Game/Lesson5/25D/BP_25DPlayer` OtherActor)
  (set `self.Open` true))

(event `self.ReceiveTick`
  (params (DeltaSeconds :type "Float (single-precision)"))
  (bind _target (`self.Target`))
  (bind _returnvalue_roll (`KismetMathLibrary.BreakRotator` (`self.K2_GetActorRotation` _target)))
  (if (`self.Open`)
    (if (> _returnvalue_roll -90.0)
      (for _ (range 91)
        (`KismetSystemLibrary.Delay` 0.001)
        (`self.K2_AddActorWorldRotation` _target (struct :`Roll` 1.0) false false))
      (else
        (`/Engine/EditorBlueprintResources/StandardMacros.DoOnce` false
          (:`Completed`
            (`self.K2_AddActorWorldOffset` (`self.Note`) (0.0 0.0 100.0) false false)
            (bind _outactors (`GameplayStatics.GetAllActorsOfClass` "/Game/Lesson5/25D/Blueprints/BP_LeftShiftText.BP_LeftShiftText_C"))
            (`self.SetActorHiddenInGame` _outactors false)
            (`KismetSystemLibrary.Delay` 3.0)
            (`self.SetActorHiddenInGame` _outactors true)))))))

(fn `UserConstructionScript`)