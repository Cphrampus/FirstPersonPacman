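; BP_Item is a collectible item for the 2.5D player that can also be thrown.
; Overlapping BP_25DPlayer while not thrown increments the player's Items count and destroys the actor.
; Throwing sets a flag and destroys it after a delay, or sooner if it drops below a height threshold.
; While thrown, Tick offsets the mesh along the player's current forward vector without sweep, leaving the stored Direction unused.
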(event `self.ReceiveBeginPlay`)

(event `self.ReceiveActorBeginOverlap`
  (params (OtherActor :type "Actor Object Reference"))
  (if (not (`self.isThrown`))
    (bind _asbp_25dplayer (cast `/Game/Lesson5/25D/BP_25DPlayer` OtherActor))
    (set `/Game/Lesson5/25D/BP_25DPlayer.Items` (+ (`/Game/Lesson5/25D/BP_25DPlayer.Items` _asbp_25dplayer) 1) _asbp_25dplayer)
    (`self.K2_DestroyActor`)))

(event `self.ReceiveTick`
  (params (DeltaSeconds :type "Float (single-precision)"))
  (bind (_returnvalue_x _returnvalue_y _returnvalue_z) (`KismetMathLibrary.BreakVector` (`self.K2_GetActorLocation`)))
  (if (`self.isThrown`)
    (if (< _returnvalue_z 1000.0)
      (`self.K2_DestroyActor`)
      (else
        (`SceneComponent.K2_AddWorldOffset` (`self.StaticMesh`) (* (`self.GetActorForwardVector` (`GameplayStatics.GetPlayerPawn` 0)) 10.0) false false)))))

(event `throw`
  (set `self.Direction` (`self.GetActorForwardVector` (`GameplayStatics.GetPlayerPawn` 0)))
  (set `self.isThrown` true)
  (`KismetSystemLibrary.Delay` 2.0)
  (`self.K2_DestroyActor`))

(fn `UserConstructionScript`)